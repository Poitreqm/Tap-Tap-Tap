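; BP_Block is a short-lived scrolling obstacle that shifts its Arrow component up by a random height on spawn and destroys itself after five seconds.
; Each tick moves the Arrow along negative X by adding DeltaSeconds to a constant rather than multiplying, so speed depends on frame rate.
; The Point overlap event is empty; logic to award points through BP_Game_Mode and destroy Point is disconnected and never runs.
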(event `self.ReceiveBeginPlay`
  (`SceneComponent.K2_SetWorldLocation` (`self.Arrow`) (+ (`SceneComponent.K2_GetComponentLocation` (`self.Arrow`)) (`KismetMathLibrary.MakeVector` 0.0 0.0 (`KismetMathLibrary.RandomFloatInRange` 170.0 50.0))) false false)
  (`KismetSystemLibrary.Delay` 5.0)
  (`self.K2_DestroyActor`))

(event `self.ReceiveTick`
  (params (DeltaSeconds :type "Float (single-precision)"))
  (`SceneComponent.K2_SetWorldLocation` (`self.Arrow`) (+ (`SceneComponent.K2_GetComponentLocation` (`self.Arrow`)) (`KismetMathLibrary.MakeVector` (+ DeltaSeconds -2.0))) false false))

(event `self.Point.OnComponentBeginOverlap`
  (params (OverlappedComponent :type "PrimitiveComponent Object Reference") (OtherActor :type "Actor Object Reference") (OtherComp :type "PrimitiveComponent Object Reference") (OtherBodyIndex :type Integer) (bFromSweep :type Boolean) (SweepResult :type "HitResult Structure (by ref)")))

(fn `UserConstructionScript`)