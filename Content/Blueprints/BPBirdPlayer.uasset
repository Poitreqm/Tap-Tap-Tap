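; Player bird for a Flappy Bird-style game, driven by capsule physics with gravity held off until the first Jump press.
; Each jump resets the capsule's velocity and applies an upward force.
; "Point"-tagged overlaps add score through BP_Game_Mode; any other kills the bird with a hop and spin, then reloads MainLevel after a delay.
; Jump while dead also reloads it; the ReadyToReastart check is unconnected.
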(event `self.ReceiveBeginPlay`
  ;[1 1 1] Gravity on if we start a game
  (`PrimitiveComponent.SetEnableGravity` (`self.Capsule`) false))

(event `self.Capsule.OnComponentBeginOverlap`
  (params (OverlappedComponent :type "PrimitiveComponent Object Reference") (OtherActor :type "Actor Object Reference") (OtherComp :type "PrimitiveComponent Object Reference") (OtherBodyIndex :type Integer) (bFromSweep :type Boolean) (SweepResult :type "HitResult Structure (by ref)"))
  (`/Engine/EditorBlueprintResources/StandardMacros.IsValid` OtherComp
    (:`Is Valid`
      (if (`ActorComponent.ComponentHasTag` OtherComp "Point")
        ;[1 1 1] Add points
        (`KismetSystemLibrary.Delay` 0.2)
        (bind _asbp_game_mode (cast `/Game/Blueprints/BP_Game_Mode` (`GameplayStatics.GetGameMode`)))
        (`/Game/Blueprints/BP_Game_Mode.AddPoints` _asbp_game_mode)
        (else
          ;[1 1 1] When we die, we make jump, rotation and our character fall
          (if (`self.isAlive`)
            (set `self.isAlive` false)
            (`self.JumpFunction`)
            (`PrimitiveComponent.AddTorqueInDegrees` (`self.Capsule`) (0.0 99999.0 0.0) "None" false)
            (`KismetSystemLibrary.Delay` 0.5)
            (`SceneComponent.K2_SetWorldLocation` (`self.Capsule`) (+ (`SceneComponent.K2_GetComponentLocation` (`self.Capsule`)) (0.0 -10.0 0.0)) false false)
            (set `self.readyToReastart` true)
            (`GameplayStatics.OpenLevel` "MainLevel")))))))

(event `InputAction|Jump`
  (params (Key :type "Key Structure"))
  (:`Pressed`
    ;[1 1 1] Start Gravity and Jump functions if we start a game
    (if (not (`self.isPlaying`))
      (set `self.isPlaying` true)
      (`PrimitiveComponent.SetEnableGravity` (`self.Capsule`) true))
    (if (`self.isAlive`)
      (`self.JumpFunction`)
      (else
        (`KismetSystemLibrary.Delay` 0.1)
        (`GameplayStatics.OpenLevel` "MainLevel")))))

(fn `JumpFunction`
  (bind _capsule (`self.Capsule`))
  (`PrimitiveComponent.SetPhysicsLinearVelocity` _capsule (1.0 -0.1 -0.1) false "None")
  (`PrimitiveComponent.AddForce` _capsule (0.0 0.0 3500.0) "None" false))

(fn `UserConstructionScript`)