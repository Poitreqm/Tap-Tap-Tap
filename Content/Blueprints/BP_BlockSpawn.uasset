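; BP_BlockSpawn is a spawner actor that keeps creating BP_Block obstacles while the bird player's game is running.
; It caches the BPBirdPlayer pawn on begin overlap, or from Tick whenever that reference is invalid.
; While IsPlaying is true, Tick runs through a one-second Delay, which throttles spawning to about one block per second at the PaperTileMap's world transform.
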(event `self.ReceiveActorBeginOverlap`
  (params (OtherActor :type "Actor Object Reference"))
  (bind _asbpbird_player (cast `/Game/Blueprints/BPBirdPlayer` (`GameplayStatics.GetPlayerPawn` 0) :!label _label)
    (:`then`
      (set `self.Player` _asbpbird_player))
    (:`CastFailed`
      (`KismetSystemLibrary.PrintString` "NOT CAST TO BIRD"))))

(event `self.ReceiveTick`
  (params (DeltaSeconds :type "Float (single-precision)"))
  (bind _player (`self.Player`))
  ;[1 1 1] Verification if we start the game
  (`/Engine/EditorBlueprintResources/StandardMacros.IsValid` _player
    (:`Is Valid`
      ;[1 1 1] Start auto-creation a blocks
      (if (`/Game/Blueprints/BPBirdPlayer.isPlaying` _player)
        (`KismetSystemLibrary.Delay` 1.0)
        (`|SpawnActorFromClass` "/Game/Blueprints/BP_Block.BP_Block_C" (`SceneComponent.K2_GetComponentToWorld` (`self.PaperTileMap`)) "Undefined" "MultiplyWithRoot" null null)))
    (:`Is Not Valid`
      (goto _label))))

(fn `UserConstructionScript`)